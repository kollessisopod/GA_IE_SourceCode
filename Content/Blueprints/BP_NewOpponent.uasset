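; AI enemy that runs a behavior tree, stores pawns it sees as the Protag blackboard key, and melees the first-person character.
; Damage lowers health and drives a dynamic material's parameters, destroying it at zero; brief invulnerability follows hits leaving health above the low-health emissive threshold.
; Attacking waits briefly, then sphere-traces between two boxes to apply damage and play a sound.
; A separate box flags player overlap.
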(event OnComponentBeginOverlap(Box)
  (params (OverlappedComponent :type Primitive%20Component%20Object%20Reference) (OtherActor :type Actor%20Object%20Reference) (OtherComp :type Primitive%20Component%20Object%20Reference) (OtherBodyIndex :type Integer) (bFromSweep :type Boolean) (SweepResult :type Hit%20Result%20Structure%20%28by%20ref%29))
  (Utilities|Casting|CastToBP_FirstPersonCharacter OtherActor)
  (Variables|Default|SetProtagOverlapping true))

(event OnComponentEndOverlap(Box)
  (params (OverlappedComponent :type Primitive%20Component%20Object%20Reference) (OtherActor :type Actor%20Object%20Reference) (OtherComp :type Primitive%20Component%20Object%20Reference) (OtherBodyIndex :type Integer))
  (Utilities|Casting|CastToBP_FirstPersonCharacter OtherActor)
  (Variables|Default|SetProtagOverlapping false))

(event OnSeePawn(PawnSensing)
  (params (Pawn :type Pawn%20Object%20Reference))
  (AI|Components|Blackboard|SetValueasObject (AI|GetBlackboard 0) (Utilities|Name|MakeLiteralName "Protag") Pawn))

(event Custom|Attacking
  (Utilities|FlowControl|Delay 0.4)
  (bind _outhit (Collision|SphereTraceForObjects (Transformation|GetWorldLocation (Variables|Default|GetBox2)) (Transformation|GetWorldLocation (Variables|Default|GetBox1)) 6e+01 (Utilities|Array|MakeArray "ObjectTypeQuery3") false 0 "ForDuration"))
  (bind _asbp_first_person_character (Utilities|Casting|CastToBP_FirstPersonCharacter (.HitActor (Collision|BreakHitResult _outhit))))
  (Game|Damage|ApplyDamage _asbp_first_person_character 1.0 0 0)
  (Audio|PlaySoundatLocation "/Engine/EditorSounds/GamePreview/EndPlayInEditor.EndPlayInEditor" (.ImpactPoint (Collision|BreakHitResult _outhit)) "0, 0, 0" 1.0 1.0 0.0 0 0 0 0))

(event EventBeginPlay
  (AI|RunBehaviorTree (AI|GetAIController self) "/Game/Blueprints/NewBehaviorTree.NewBehaviorTree"))

(event Game|Damage|EventAnyDamage
  (params (Damage :type Float%20%28single-precision%29) (DamageType :type Damage%20Type%20Object%20Reference) (InstigatedBy :type Controller%20Object%20Reference) (DamageCauser :type Actor%20Object%20Reference))
  (bind _materialinstance (Variables|Default|GetMaterialInstance))
  (if (not (Variables|Default|GetInvulnerability))
    (bind _output_get (Variables|Default|SetEnemyHealth (- (Variables|Default|GetEnemyHealth) Damage)))
    (if (> _output_get 0.0)
      (Rendering|Material|SetScalarParameterValue _materialinstance "ParameterYum" (/ _output_get 51.0) :!class /Script/Engine.MaterialInstanceDynamic)
      (if (<= (Variables|Default|GetEnemyHealth) 2e+01)
        (Rendering|Material|SetScalarParameterValue _materialinstance "Emissive" 0.2 :!class /Script/Engine.MaterialInstanceDynamic)
        (else
          (Variables|Default|SetInvulnerability true :!label _label)
          (Utilities|FlowControl|Delay 0.2)
          (Variables|Default|SetInvulnerability false)))
      (else
        (Actor|DestroyActor)
        (goto _label)))))

(fn ConstructionScript
  (bind _returnvalue (Rendering|Material|CreateDynamicMaterialInstance (Variables|Character|GetMesh) 0 "/Game/Blueprints/Materials/Material_Deneme1.Material_Deneme1" "None" :!class /Script/Engine.PrimitiveComponent))
  (bind _output_get (Variables|Default|SetMaterialInstance _returnvalue))
  (Rendering|Material|SetMaterial (Variables|Character|GetMesh) 0 _output_get))