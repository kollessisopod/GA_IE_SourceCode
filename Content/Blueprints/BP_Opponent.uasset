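; BP_Opponent is a damageable opponent actor that loses Health and is destroyed when it reaches zero.
; AnyDamage subtracts damage unless IsInvulnerable is set, printing the remaining health or a death message as debug output.
; Each accepted hit then sets a brief invulnerability window through a Delay, so rapid repeated hits are ignored.
; BeginPlay, overlap, Tick and the construction script are empty.
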(event EventBeginPlay)

(event Collision|EventActorBeginOverlap
  (params (OtherActor :type Actor%20Object%20Reference)))

(event EventTick
  (params (DeltaSeconds :type Float%20%28single-precision%29)))

(event Game|Damage|EventAnyDamage
  (params (Damage :type Float%20%28single-precision%29) (DamageType :type Damage%20Type%20Object%20Reference) (InstigatedBy :type Controller%20Object%20Reference) (DamageCauser :type Actor%20Object%20Reference))
  (if (not (Variables|Default|GetIsInvulnerable))
    (bind _output_get (Variables|Default|SetHealth (- (Variables|Default|GetHealth) Damage)))
    (if (> _output_get 0.0)
      (Development|PrintString "HEALTH DROPPED TO:")
      (Development|PrintString (Utilities|String|ToString(Float) _output_get))
      (else
        (Actor|DestroyActor)
        (Development|PrintString "DEADL MAO")))
    (Variables|Default|SetIsInvulnerable true)
    (Utilities|FlowControl|Delay 0.2)
    (Variables|Default|SetIsInvulnerable false)))

(fn ConstructionScript)